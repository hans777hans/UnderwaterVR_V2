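; BP_Skybox is a skybox actor whose static mesh can switch between six sky materials.
; ChangeMaterial takes an index, applies the matching M_Skybox material to element 0 as a new dynamic instance, and returns the corresponding entry from a string array.
; The construction script applies the first material by default, and the event graph holds no active logic, so any later switching must come from an external caller.
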(fn `ChangeMaterial`
  (params (IndexInt :type Integer))
  (returns (ReturnStr :type String))
  (bind _staticmesh (`self.StaticMesh`))
  (switch `int` IndexInt
    (:`0`
      (`PrimitiveComponent.CreateDynamicMaterialInstance` _staticmesh 0 "/Game/Materials/M_Skybox1.M_Skybox1")
      (return (`|GetArrayItem` (`self.StringArray`))))
    (:`1`
      (`PrimitiveComponent.CreateDynamicMaterialInstance` _staticmesh 0 "/Game/Materials/M_Skybox2.M_Skybox2")
      (return (`|GetArrayItem` (`self.StringArray`) 1)))
    (:`2`
      (`PrimitiveComponent.CreateDynamicMaterialInstance` _staticmesh 0 "/Game/Materials/M_Skybox3.M_Skybox3")
      (return (`|GetArrayItem` (`self.StringArray`) 2)))
    (:`3`
      (`PrimitiveComponent.CreateDynamicMaterialInstance` _staticmesh 0 "/Game/Materials/M_Skybox4.M_Skybox4")
      (return (`|GetArrayItem` (`self.StringArray`) 3)))
    (:`4`
      (`PrimitiveComponent.CreateDynamicMaterialInstance` _staticmesh 0 "/Game/Materials/M_Skybox5.M_Skybox5")
      (return (`|GetArrayItem` (`self.StringArray`) 4)))
    (:`5`
      (`PrimitiveComponent.CreateDynamicMaterialInstance` _staticmesh 0 "/Game/Materials/M_Skybox6.M_Skybox6")
      (return (`|GetArrayItem` (`self.StringArray`) 5)))))

(fn `UserConstructionScript`
  (`self.ChangeMaterial` 0))