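; BP_GreenSphere is an interactive sphere that turns red on focus, green on blur and blue on activation, via interface events.
; Activation gets the next skybox index from GetNextValidIndex, which wraps past a fixed limit, then messages BPSkyboxRef to change material.
; It prints the index and the matching name from BP_Skybox's default string array.
; An overlap event assigns BPSkyboxRef and re-enters that change step, but the cast supplying the reference never executes.
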(event OnActorBeginOverlap(BPSkybox_Ref)
  (params (OverlappedActor :type Actor%20Object%20Reference) (OtherActor :type Actor%20Object%20Reference))
  ;[1 1 1] Green Sphere Interface Implementations
  (bind _output_get (Variables|Default|SetBPSkybox_Ref (stale _asbp_skybox)))
  (Class|BPIMaterial|ChangeMaterial(Message) _output_get (stale EventOnActivate _outputindex))
  (Development|PrintString (Utilities|Array|Get(acopy) (.StringArray (Utilities|GetClassDefaults "/Game/Blueprints/BP_Skybox.BP_Skybox_C")) (stale EventOnActivate _outputindex)) true true "(R=0.052770,G=0.870242,B=1.000000,A=1.000000)"))

(event EventOnBlur
  ;[1 1 1] Green Sphere Interface Implementations
  (Rendering|Material|SetMaterial (Variables|Default|GetSphere) 0 "/Game/Materials/M_Green.M_Green"))

(event EventOnFocus
  ;[1 1 1] Green Sphere Interface Implementations
  (Rendering|Material|SetMaterial (Variables|Default|GetSphere) 0 "/Game/Materials/M_Red.M_Red"))

(event EventOnActivate
  ;[1 1 1] Green Sphere Interface Implementations
  (Rendering|Material|SetMaterial (Variables|Default|GetSphere) 0 "/Game/Materials/M_Blue.M_Blue")
  (bind _outputindex (CallFunction|GetNextValidIndex))
  (Development|PrintString (Utilities|String|ToString(Integer) _outputindex))
  (Class|BPIMaterial|ChangeMaterial(Message) (stale OnActorBeginOverlap(BPSkybox_Ref) _output_get) _outputindex)
  (Development|PrintString (Utilities|Array|Get(acopy) (.StringArray (Utilities|GetClassDefaults "/Game/Blueprints/BP_Skybox.BP_Skybox_C")) _outputindex) true true "(R=0.052770,G=0.870242,B=1.000000,A=1.000000)"))

(fn ConstructionScript)

(fn GetNextValidIndex
  (bind _result (Math|Integer|IncrementInt (Variables|Default|GetSkyboxIndex))
    (:%20%20
      (if (<= _result 5)
        (return _result)
        (else
          (bind _output_get (Variables|Default|SetSkyboxIndex (Variables|Default|GetZeroIndex)))
          (return _output_get))))))