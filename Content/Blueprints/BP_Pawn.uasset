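; Pawn that provides gaze-based interaction, letting the player focus and activate actors by looking at them.
; Each tick it line traces on the Visibility channel along the camera's forward vector.
; When the hit actor changes, it sends blur to the previous InteractiveActor and focus to the new one through message calls.
; A fixed Delay then sends activate to whichever actor is current when it expires, as gaze changes do not cancel it.
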(event `self.ReceiveTick`
  (params (DeltaSeconds :type "Float (single-precision)"))
  ;[1 1 1] Gaze Check - Gaze tracking interaction
  (`self.GazeCheck`))

(event `GazeCheck`
  (bind _camera (`self.Camera`))
  (bind _returnvalue (`SceneComponent.K2_GetComponentLocation` _camera))
  ;[1 1 1] Gaze Check - Gaze tracking interaction
  (bind _outhit (`KismetSystemLibrary.LineTraceSingle` :`Start` _returnvalue :`End` (+ _returnvalue (* (`SceneComponent.GetForwardVector` _camera) 2000.0)) :`TraceChannel` "TraceTypeQuery1" :`TraceColor` (struct :`R` 1.0 :`G` 1.0 :`B` 1.0 :`A` 1.0)))
  (bind (_bblockinghit _binitialoverlap _time _location _impactpoint _normal _impactnormal _physmat _hitactor) (`GameplayStatics.BreakHitResult` _outhit))
  (if (!= _hitactor (`self.InteractiveActor`))
    (message `/Game/Blueprints/BPI_Interaction.OnBlur` (`self.InteractiveActor`))
    (bind _output_get (set `self.InteractiveActor` _hitactor))
    (message `/Game/Blueprints/BPI_Interaction.OnFocus` _output_get)
    (`KismetSystemLibrary.Delay` 5.0)
    (message `/Game/Blueprints/BPI_Interaction.OnActivate` _output_get)))

(fn `UserConstructionScript`)